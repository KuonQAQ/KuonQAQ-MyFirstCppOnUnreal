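; BP_EnemyBase is an enemy base Blueprint that handles burning visuals and damage feedback.
; Each Tick it checks the action component's active gameplay tags for Status.Buring and activates or deactivates the PBurning effect to match.
; When the attribute component reports a health change, it creates a WB_DamagePOp widget attached to itself with the delta and adds it to the viewport.
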(event OnHealthChanged(AttributeComponent)
  (params (InstigatorActor :type Actor%20Object%20Reference) (OwningComp :type Attribute%20Component%20Object%20Reference) (NewHealth :type Float%20%28single-precision%29) (Delta :type Float%20%28single-precision%29))
  (bind _returnvalue (UserInterface|CreateWidget "/Game/FcppProject/BluePrint/UI/WB_DamagePOp.WB_DamagePOp_C" 0 self Delta))
  (UserInterface|Viewport|AddtoViewport _returnvalue 0))

(event EventBeginPlay)

(event Collision|EventActorBeginOverlap
  (params (OtherActor :type Actor%20Object%20Reference)))

(event EventTick
  (params (DeltaSeconds :type Float%20%28single-precision%29))
  (bind _p_burning (Variables|Default|GetP_Burning))
  (if (GameplayTags|HasTag (Variables|/Script/FcppProject.LActionComponent|GetActiveGameplayTags (Variables|Default|GetLAction)) "(TagName=\"Status.Buring\")" true)
    (Components|Activation|Activate _p_burning false)
    (else
      (Components|Activation|Deactivate _p_burning))))

(fn ConstructionScript)